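; MainHUD is a poker HUD that draws the owning player's starting hand and the betting key prompts on screen.
; Each DrawHUD call casts the owning controller's PlayerState to MainPlayerState and prints the number and pattern of Card1 and Card2 with DrawText.
; PlayerId parity selects whether number keys or QWER are shown for Call, Raise, Fold and Check.
; DrawCardInfo and the other events are empty.
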(event `self.ReceiveDrawHUD`
  (params (SizeX :type Integer) (SizeY :type Integer))
  (bind _playerstate (`Controller.PlayerState` (`self.GetOwningPlayerController`)))
  (bind _asmain_player_state (cast `/Game/Blueprints/MainPlayerState` _playerstate))
  (`|ExecutionSequence`
    (:`then_0`
      (`|ExecutionSequence`
        (:`then_0`
          (`self.DrawText` "Press the action key" (struct :`R` 1.0 :`A` 1.0) 250.0 80.0))
        (:`then_1`
          (if (== (mod (`PlayerState.PlayerId` _playerstate) 2) 0)
            (`self.DrawText` "1 : Call  2 : Raise  3 : Fold 4 : Check" (struct :`A` 1) 250.0 100.0)
            (else
              (`self.DrawText` "Q  : Call  W : Raise  E : Fold R : Check" (struct :`A` 1) 250.0 100.0))))
        (:`then_2`
          (`self.DrawText` "It's your starting hands" (struct :`A` 1) 10.0 80.0 null 1.25))))
    (:`then_1`
      (bind _card1 (`/Game/Blueprints/MainPlayerState.card1` _asmain_player_state))
      (bind _returnvalue (`Card.GetNum` _card1))
      (`self.DrawText` (`KismetStringLibrary.Conv_IntToString` _returnvalue) (struct :`A` 1.0) 90.0 105.0 null 1.0))
    (:`then_2`
      (bind _returnvalue_2 (`Card.GetPattern` _card1))
      (`self.DrawText` (`|GetEnumeratorNameAsString` _returnvalue_2) (struct :`A` 1) 10.0 105.0))
    (:`then_3`
      (`|ExecutionSequence`
        (:`then_0`
          (bind _card2 (`/Game/Blueprints/MainPlayerState.card2` _asmain_player_state))
          (bind _returnvalue_3 (`Card.GetNum` _card2))
          (`self.DrawText` (`KismetStringLibrary.Conv_IntToString` _returnvalue_3) (struct :`A` 1.0) 90.0 125.0 null 1.0))
        (:`then_1`
          (bind _returnvalue_4 (`Card.GetPattern` _card2))
          (`self.DrawText` (`|GetEnumeratorNameAsString` _returnvalue_4) (struct :`A` 1) 10.0 125.0))))))

(event `self.ReceiveBeginPlay`)

(fn `DrawCardInfo`
  (params (MainHUD :type "/Game/Blueprints/MainHUD Object Reference")))

(fn `UserConstructionScript`)