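; HUD Blueprint that manages a player's game-info widget and turn-based action widget.
; On BeginPlay it creates both widgets for the owning controller and adds only the game-info widget, stored as HandWidget, to the player screen.
; Tick polls MyTurn on TH_PlayerState and uses the IsShown flag to add or remove the action widget only on changes, with debug prints.
; DrawHUD and DrawCardInfo are empty.
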(event `self.ReceiveBeginPlay`
  (bind _returnvalue (`self.GetOwningPlayerController`))
  (set `self.isShown` false)
  (bind _returnvalue_2 (`|CreateWidget` "/Game/Blueprints/PlayerActionWidget.PlayerActionWidget_C" _returnvalue))
  (set `self.actionWidget` _returnvalue_2)
  (bind _returnvalue_3 (`|CreateWidget` "/Game/Blueprints/GameInfoWidget.GameInfoWidget_C" _returnvalue))
  (bind _output_get (set `self.handWidget` _returnvalue_3))
  (`UserWidget.AddToPlayerScreen` _output_get 0))

(event `self.ReceiveDrawHUD`
  (params (SizeX :type Integer) (SizeY :type Integer)))

(event `self.ReceiveTick`
  (params (DeltaSeconds :type "Float (single-precision)"))
  (bind _actionwidget (`self.actionWidget`))
  (bind _asth_player_state (cast `/Game/Blueprints/TH_PlayerState` (`Controller.PlayerState` (`self.GetOwningPlayerController`))))
  (if (`/Game/Blueprints/TH_PlayerState.myTurn` _asth_player_state)
    (if (not (`self.isShown`))
      (set `self.isShown` true)
      (`KismetSystemLibrary.PrintString` "Hello")
      (`UserWidget.AddToPlayerScreen` _actionwidget 0))
    (elif (`self.isShown`)
      (set `self.isShown` false)
      (`KismetSystemLibrary.PrintString` "remove")
      (`Widget.RemoveFromParent` _actionwidget))))

(fn `DrawCardInfo`
  (params (MainHUD :type "/Game/Blueprints/TH_HUD Object Reference")))

(fn `UserConstructionScript`)