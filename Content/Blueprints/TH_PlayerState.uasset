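; Player state for a hole-card game that copies the player's two cards and gates input to their turn.
; Tick derives a seat index from PlayerId and pulls Card1 and Card2 from TH_GameState after a short delay, then sets its shared IsHoleCardSpread flag.
; It also compares the seat with Turn, toggles input on the first player controller's TH_Pawn, and calls PassTurn once that pawn has acted.
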(event `self.ReceiveBeginPlay`)

(event `self.ReceiveTick`
  (params (DeltaSeconds :type "Float (single-precision)"))
  (`|ExecutionSequence`
    (:`then_0`
      (bind _asth_game_state (cast `TH_GameState` (`GameplayStatics.GetGameState`)))
      (if (not (`TH_GameState.isHoleCardSpread` _asth_game_state))
        (`KismetSystemLibrary.PrintString` "PlayerState")
        (`KismetSystemLibrary.Delay` 0.1)
        (bind _asth_game_state_2 (cast `TH_GameState` (`GameplayStatics.GetGameState`)))
        (bind _returnvalue (mod (+ (`self.PlayerId`) 1) (`TH_GameState.numTotalPlayer` _asth_game_state_2)))
        (bind _returnvalue_2 (`TH_GameState.GetPlayerHands` _asth_game_state_2 _returnvalue 0))
        (set `self.card1` _returnvalue_2)
        (bind _returnvalue_3 (`TH_GameState.GetPlayerHands` _asth_game_state_2 _returnvalue 1))
        (set `self.card2` _returnvalue_3)
        (set `TH_GameState.isHoleCardSpread` true _asth_game_state)))
    (:`then_1`
      (bind _asth_game_state_3 (cast `TH_GameState` (`GameplayStatics.GetGameState`)))
      (bind _returnvalue_4 (mod (+ (`self.PlayerId`) 1) (`TH_GameState.numTotalPlayer` _asth_game_state_3)))
      (bind _output_get (set `self.myTurn` (== (`TH_GameState.turn` _asth_game_state_3) _returnvalue_4)))
      (set `self.index` _returnvalue_4)
      (bind _returnvalue_5 (`TH_Pawn.GetPlayerController` self))
      (if _output_get
        (bind _returnvalue_6 (`Controller.K2_GetPawn` _returnvalue_5))
        (`self.EnableInput` _returnvalue_6 _returnvalue_5)
        (bind _asth_pawn (cast `TH_Pawn` _returnvalue_6))
        (set `TH_Pawn.is_tick_start` true _asth_pawn)
        (bind _returnvalue_7 (`TH_Pawn.GetActed` _asth_pawn))
        (if _returnvalue_7
          (bind _asth_game_state_4 (cast `TH_GameState` (`GameplayStatics.GetGameState`)))
          (`TH_GameState.PassTurn` _asth_game_state_4)
          (`TH_Pawn.SetActed` _asth_pawn false)
          (set `TH_Pawn.is_tick_start` false _asth_pawn))
        (else
          (`self.DisableInput` _returnvalue_6 _returnvalue_5)
          (bind _asth_pawn_2 (cast `TH_Pawn` _returnvalue_6))
          (set `TH_Pawn.is_tick_start` false _asth_pawn_2))))))

(fn `UserConstructionScript`)